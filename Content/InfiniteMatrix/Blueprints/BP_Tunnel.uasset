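; BP_Tunnel is a tunnel segment for an endless game, with a rotating wall, randomly offset and shown health pack and enemy.
; Entering TriggerZone asks TunnelSpawner for a new segment and destroys this one.
; Component overlaps adjust BP_Player health and score, triggering restart display on death, while enemies are destroyed by player or BP_ProjectileSpawner contact.
; RandomizeWall, uncalled here, picks one of four hole meshes and a random roll.
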(event OnComponentBeginOverlap(WallMesh)
  (params (OverlappedComponent :type Primitive%20Component%20Object%20Reference) (OtherActor :type Actor%20Object%20Reference) (OtherComp :type Primitive%20Component%20Object%20Reference) (OtherBodyIndex :type Integer) (bFromSweep :type Boolean) (SweepResult :type Hit%20Result%20Structure%20%28by%20ref%29))
  (Utilities|FlowControl|Sequence
    (:then_0
      (bind _asbp_player (Utilities|Casting|CastToBP_Player OtherActor))
      (bind _output_get (Variables|/Game/InfiniteMatrix/Blueprints/BP_Player.BP_Player_C|SetHealth _asbp_player (- (Variables|/Game/InfiniteMatrix/Blueprints/BP_Player.BP_Player_C|GetHealth _asbp_player) 10)))
      (if (<= _output_get 0)
        (Variables|/Game/InfiniteMatrix/Blueprints/BP_Player.BP_Player_C|SetisDead _asbp_player true)
        (Variables|Default|SetRotateSpeed 0.0)
        (Default|DisplayRestart _asbp_player)))))

(event OnComponentBeginOverlap(HealthPack)
  (params (OverlappedComponent :type Primitive%20Component%20Object%20Reference) (OtherActor :type Actor%20Object%20Reference) (OtherComp :type Primitive%20Component%20Object%20Reference) (OtherBodyIndex :type Integer) (bFromSweep :type Boolean) (SweepResult :type Hit%20Result%20Structure%20%28by%20ref%29))
  (Utilities|FlowControl|Sequence
    (:then_0
      (bind _asbp_player (Utilities|Casting|CastToBP_Player OtherActor))
      (Variables|/Game/InfiniteMatrix/Blueprints/BP_Player.BP_Player_C|SetHealth _asbp_player (Math|Integer|Clamp(Integer) (+ (Variables|/Game/InfiniteMatrix/Blueprints/BP_Player.BP_Player_C|GetHealth _asbp_player) 10) 0 100)))))

(event OnComponentBeginOverlap(TriggerZone)
  (params (OverlappedComponent :type Primitive%20Component%20Object%20Reference) (OtherActor :type Actor%20Object%20Reference) (OtherComp :type Primitive%20Component%20Object%20Reference) (OtherBodyIndex :type Integer) (bFromSweep :type Boolean) (SweepResult :type Hit%20Result%20Structure%20%28by%20ref%29))
  (Utilities|FlowControl|Sequence
    (:then_0
      (Utilities|Casting|CastToBP_Player OtherActor)
      (Default|SpawnTunnelatSpawnPoint (Variables|Default|GetTunnelSpawner))
      (Actor|DestroyActor))))

(event OnComponentBeginOverlap(Enemy)
  (params (OverlappedComponent :type Primitive%20Component%20Object%20Reference) (OtherActor :type Actor%20Object%20Reference) (OtherComp :type Primitive%20Component%20Object%20Reference) (OtherBodyIndex :type Integer) (bFromSweep :type Boolean) (SweepResult :type Hit%20Result%20Structure%20%28by%20ref%29))
  (bind _enemy (Variables|Default|GetEnemy))
  (bind _enemy_2 (Variables|Default|GetEnemy))
  (bind _bp_playerref (Variables|Default|GetBP_PlayerRef))
  (Utilities|FlowControl|Sequence
    (:then_0
      (bind _asbp_player (Utilities|Casting|CastToBP_Player OtherActor))
      (bind _output_get (Variables|/Game/InfiniteMatrix/Blueprints/BP_Player.BP_Player_C|SetHealth _asbp_player (- (Variables|/Game/InfiniteMatrix/Blueprints/BP_Player.BP_Player_C|GetHealth _asbp_player) 10)))
      (if (<= _output_get 0)
        (Variables|/Game/InfiniteMatrix/Blueprints/BP_Player.BP_Player_C|SetisDead _asbp_player true)
        (Variables|Default|SetRotateSpeed 0.0)
        (Default|DisplayRestart _asbp_player)))
    (:then_1
      (Utilities|FlowControl|Sequence
        (:then_0
          (Utilities|Casting|CastToBP_ProjectileSpawner OtherActor)
          (Utilities|IsValid _enemy_2
            (:Is%20Valid
              (Components|DestroyComponent _enemy_2))))
        (:then_1
          (Utilities|Casting|CastToBP_Player OtherActor)
          (Utilities|IsValid _enemy
            (:Is%20Valid
              (Components|DestroyComponent _enemy))))))
    (:then_2
      (Utilities|Casting|CastToBP_ProjectileSpawner OtherActor)
      (Utilities|IsValid _bp_playerref
        (:Is%20Valid
          (Variables|/Game/InfiniteMatrix/Blueprints/BP_Player.BP_Player_C|SetScore _bp_playerref (Math|Integer|Clamp(Integer) (+ (Variables|/Game/InfiniteMatrix/Blueprints/BP_Player.BP_Player_C|GetScore _bp_playerref) 10) 0 10000)))))))

(event OnComponentEndOverlap(WallMesh)
  (params (OverlappedComponent :type Primitive%20Component%20Object%20Reference) (OtherActor :type Actor%20Object%20Reference) (OtherComp :type Primitive%20Component%20Object%20Reference) (OtherBodyIndex :type Integer))
  (bind _asbp_player (Utilities|Casting|CastToBP_Player OtherActor))
  (Variables|/Game/InfiniteMatrix/Blueprints/BP_Player.BP_Player_C|SetScore _asbp_player (Math|Integer|Clamp(Integer) (- (Variables|/Game/InfiniteMatrix/Blueprints/BP_Player.BP_Player_C|GetScore _asbp_player) 10) 0 10000)))

(event OnComponentEndOverlap(TriggerZone)
  (params (OverlappedComponent :type Primitive%20Component%20Object%20Reference) (OtherActor :type Actor%20Object%20Reference) (OtherComp :type Primitive%20Component%20Object%20Reference) (OtherBodyIndex :type Integer))
  (bind _asbp_player (Utilities|Casting|CastToBP_Player OtherActor))
  (Variables|/Game/InfiniteMatrix/Blueprints/BP_Player.BP_Player_C|SetScore _asbp_player (+ (Variables|/Game/InfiniteMatrix/Blueprints/BP_Player.BP_Player_C|GetScore _asbp_player) 10)))

(event EventBeginPlay
  (bind _returnvalue (Math|Random|RandomInteger 2))
  (bind _returnvalue_2 (Math|Random|RandomInteger 7))
  (bind _staticmeshcomponent (Variables|Debug|GetStaticMeshComponent))
  (bind _healthpack (Variables|Default|GetHealthPack))
  (bind _enemy (Variables|Default|GetEnemy))
  (bind _staticmeshcomponent_2 (Variables|Debug|GetStaticMeshComponent))
  (bind (_origin _boxextent) (Collision|GetComponentBounds _staticmeshcomponent_2))
  (bind (_origin_2 _boxextent_2) (Collision|GetComponentBounds _staticmeshcomponent))
  (bind _returnvalue_3 (== _returnvalue 1))
  (bind _returnvalue_4 (== _returnvalue_2 2))
  (Utilities|FlowControl|Sequence
    (:then_0
      (if (Math|Conversions|ToBoolean(Integer) _returnvalue_2)
        (Transformation|AddLocalOffset _healthpack (Math|Vector|MakeVector (Math|Random|RandomFloatinRange (+ (- (.x _origin_2) (.x _boxextent_2)) 2.5e+02) (- (+ (.x _origin_2) (.x _boxextent_2)) 2.5e+02)) (Math|Random|RandomFloatinRange (+ (- (.y _origin_2) (.y _boxextent_2)) 2.5e+02) (- (+ (.y _origin_2) (.y _boxextent_2)) 2.5e+02)) (Math|Random|RandomFloatinRange (+ (- (.z _origin_2) (.z _boxextent_2)) 2.5e+02) (- (+ (.z _origin_2) (.z _boxextent_2)) 2.5e+02))) true false)
        (Rendering|SetVisibility _healthpack _returnvalue_4 true)
        (else
          (Rendering|SetVisibility (Variables|Default|GetHealthPack) _returnvalue_4 true))))
    (:then_1
      (if (Math|Conversions|ToBoolean(Integer) _returnvalue)
        (Transformation|AddLocalOffset _enemy (Math|Vector|MakeVector (Math|Random|RandomFloatinRange (+ (- (.x _origin) (.x _boxextent)) 3e+02) (- (+ (.x _origin) (.x _boxextent)) 3e+02)) (Math|Random|RandomFloatinRange (+ (- (.y _origin) (.y _boxextent)) 3e+02) (- (+ (.y _origin) (.y _boxextent)) 3e+02)) (Math|Random|RandomFloatinRange (+ (- (.z _origin) (.z _boxextent)) 3e+02) (- (+ (.z _origin) (.z _boxextent)) 3e+02))) true false)
        (Utilities|IsValid _enemy
          (:Is%20Valid
            (Rendering|SetVisibility _enemy _returnvalue_3 true)
            (Development|PrintString "VISIBLE")))
        (else
          (Rendering|SetVisibility (Variables|Default|GetEnemy) _returnvalue_3 true))))))

(event EventTick
  (params (DeltaSeconds :type Float%20%28single-precision%29))
  (Transformation|AddLocalRotation (Variables|Default|GetWallMesh) (Math|Rotator|MakeRotator (* DeltaSeconds (Variables|Default|GetRotateSpeed)) 0.0 0.0) false false))

(fn ConstructionScript)

(fn RandomizeWall
  (Components|StaticMesh|SetStaticMesh (Variables|Default|GetWallMesh) (Utilities|Select :Index (Math|Random|RandomIntegerinRange 0 3) :Option%200 "/Game/InfiniteMatrix/Meshes/SM_Hole_01.SM_Hole_01" :Option%201 "/Game/InfiniteMatrix/Meshes/SM_Hole_02.SM_Hole_02" :Option%202 "/Game/InfiniteMatrix/Meshes/SM_Hole_03.SM_Hole_03" :Option%203 "/Game/InfiniteMatrix/Meshes/SM_Hole_04.SM_Hole_04"))
  (Transformation|AddLocalRotation (Variables|Default|GetWallMesh) (Math|Rotator|MakeRotator (Math|Random|RandomFloatinRange 0.0 3.6e+02) 0.0 0.0) false false))

(fn DestroyHealthPackFn
  (Development|PrintString "Hello" true true "(R=0.997660,G=0.933211,B=1.000000,A=1.000000)")
  (Components|DestroyComponent (Variables|Default|GetHealthPack)))